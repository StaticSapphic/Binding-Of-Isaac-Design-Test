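; RoomManager is a Blueprint that opens a room by destroying its doors once no enemies remain.
; On BeginPlay it sets itself as Manager on each entry in its Enemies array.
; EnemyDied destroys every actor in Doors when Enemies is empty; it does not remove entries from that array itself.
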(event Custom|EnemyDied
  (if (== (Utilities|Array|Length (Variables|Default|GetEnemies)) 0)
    (for _array_element (Variables|Default|GetDoors)
      (Actor|DestroyActor _array_element))))

(event EventBeginPlay
  (for _array_element (Variables|Default|GetEnemies)
    (Variables|/Game/Blueprints/GenericEnemy.GenericEnemy_C|SetManager _array_element self)))

(fn ConstructionScript)