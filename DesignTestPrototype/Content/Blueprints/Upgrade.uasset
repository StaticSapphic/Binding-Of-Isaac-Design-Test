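; Upgrade pickup actor that improves the player's tear attack when the player character overlaps its collider.
; An Upgrade enum selects which ThirdPersonCharacter stat changes: fire delay, tear speed, damage, piercing or range, with range raised by lowering tear gravity.
; The pickup destroys itself after applying the change.
; The Construction Script sets the label text from the same enum, so each placed instance shows its type.
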(event OnComponentBeginOverlap(Collider)
  (params (OverlappedComponent :type Primitive%20Component%20Object%20Reference) (OtherActor :type Actor%20Object%20Reference) (OtherComp :type Primitive%20Component%20Object%20Reference) (OtherBodyIndex :type Integer) (bFromSweep :type Boolean) (SweepResult :type Hit%20Result%20Structure%20%28by%20ref%29))
  (bind _returnvalue (Game|GetPlayerCharacter 0))
  (if (== OtherActor _returnvalue)
    (bind _asthird_person_character (Utilities|Casting|CastToThirdPersonCharacter _returnvalue))
    (Variables|Default|SetPlayer _asthird_person_character)
    (switch Utilities|FlowControl|Switch|SwitchonUpgrades (Variables|Default|GetUpgrade)
      (:NewEnumerator0
        (Variables|/Game/Blueprints/ThirdPersonCharacter.ThirdPersonCharacter_C|SetTearDelay (Variables|Default|GetPlayer) (- (Variables|/Game/Blueprints/ThirdPersonCharacter.ThirdPersonCharacter_C|GetTearDelay (Variables|Default|GetPlayer)) 0.09)))
      (:NewEnumerator1
        (Variables|/Game/Blueprints/ThirdPersonCharacter.ThirdPersonCharacter_C|SetTearSpeed (Variables|Default|GetPlayer) (+ (Variables|/Game/Blueprints/ThirdPersonCharacter.ThirdPersonCharacter_C|GetTearSpeed (Variables|Default|GetPlayer)) 3e+02)))
      (:NewEnumerator2
        (Variables|/Game/Blueprints/ThirdPersonCharacter.ThirdPersonCharacter_C|SetDamage (Variables|Default|GetPlayer) (+ (Variables|/Game/Blueprints/ThirdPersonCharacter.ThirdPersonCharacter_C|GetDamage (Variables|Default|GetPlayer)) 2.0)))
      (:NewEnumerator3
        (Variables|/Game/Blueprints/ThirdPersonCharacter.ThirdPersonCharacter_C|SetPiercingTears (Variables|Default|GetPlayer) true))
      (:NewEnumerator5
        (Variables|/Game/Blueprints/ThirdPersonCharacter.ThirdPersonCharacter_C|SetTearGravity (Variables|Default|GetPlayer) (- (Variables|/Game/Blueprints/ThirdPersonCharacter.ThirdPersonCharacter_C|GetTearGravity (Variables|Default|GetPlayer)) 0.15))))
    (Actor|DestroyActor)))

(event EventBeginPlay)

(fn ConstructionScript
  (Rendering|Components|TextRender|SetText (Variables|Default|GetLabel) (Utilities|Select :Index (Variables|Default|GetUpgrade) :NewEnumerator0 (Utilities|Text|FormatText "Tears 
Up") :NewEnumerator1 (Utilities|Text|FormatText "Shot 
Speed Up") :NewEnumerator2 (Utilities|Text|FormatText "Damage 
Up") :NewEnumerator3 (Utilities|Text|FormatText "Piercing 
Tears") :NewEnumerator5 (Utilities|Text|FormatText "Range Up"))))