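; Generic enemy Blueprint that takes damage, dies, and hurts the player through contact.
; Damage lowers Health, then either briefly turns the mesh red with a short invulnerability window or, at zero, removes the enemy from the Manager's list, notifies it and destroys the actor.
; Player overlap with the Damage component starts a delayed loop that repeatedly applies damage while contact lasts, the delay preventing an infinite-loop error.
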(event OnComponentBeginOverlap(Damage)
  (params (OverlappedComponent :type Primitive%20Component%20Object%20Reference) (OtherActor :type Actor%20Object%20Reference) (OtherComp :type Primitive%20Component%20Object%20Reference) (OtherBodyIndex :type Integer) (bFromSweep :type Boolean) (SweepResult :type Hit%20Result%20Structure%20%28by%20ref%29))
  ;[1 1 1] Continuous contact damage
  (if (and (== OtherActor (Game|GetPlayerCharacter 0)) (Collision|IsOverlappingActor (Variables|Default|GetDamage) OtherActor :!class /Script/Engine.PrimitiveComponent)) :!label _label
    ;;[1 1 1 1 14] Required to prevent infinite loop error
    (Utilities|FlowControl|Delay 0.1)
    (Game|Damage|ApplyDamage OtherActor 1.0 0 self)
    (goto _label)))

(event Game|Damage|EventAnyDamage
  (params (Damage :type Float%20%28single-precision%29) (DamageType :type Damage%20Type%20Object%20Reference) (InstigatedBy :type Controller%20Object%20Reference) (DamageCauser :type Actor%20Object%20Reference))
  (bind _output_get (Variables|Default|SetHealth (- (Variables|Default|GetHealth) Damage)))
  (if (<= _output_get 0.0)
    (Utilities|Array|RemoveItem (Variables|/Game/Blueprints/RoomManager.RoomManager_C|GetEnemies (Variables|Default|GetManager)) self)
    (Default|EnemyDied (Variables|Default|GetManager))
    (Actor|DestroyActor)
    (else
      ;[1 1 1] Invulnerability time and material change to indicate damage
      (Variables|Actor|SetbCanBeDamaged false)
      (Rendering|Material|SetMaterial (Variables|Character|GetMesh) 0 "/Game/Materials/Red.Red")
      (Utilities|FlowControl|Delay 0.2)
      (Rendering|Material|SetMaterial (Variables|Character|GetMesh) 0 "/Game/Mannequin/Character/Materials/M_Male_Body.M_Male_Body")
      (Variables|Actor|SetbCanBeDamaged true))))

(fn ConstructionScript)