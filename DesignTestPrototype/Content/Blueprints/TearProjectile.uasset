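; TearProjectile is a tear projectile that applies point damage to any overlapping actor other than the first player's pawn.
; A Piercing flag lets it survive hits, while normal tears destroy themselves after the first one.
; The construction script hides the Cone component in game unless Piercing is set.
; Damage uses a default hit result and passes the tear's world location as the hit direction.
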(event EventBeginPlay)

(event EventTick
  (params (DeltaSeconds :type Float%20%28single-precision%29)))

(event Collision|EventActorBeginOverlap
  (params (OtherActor :type Actor%20Object%20Reference))
  (if (not (== (Game|Player|GetPlayerPawn 0) OtherActor))
    (Game|Damage|ApplyPointDamage OtherActor (Variables|Default|GetDamage) (Transformation|GetActorLocation) (Collision|MakeHitResult false false 0.0 0.0 "0, 0, 0" "0, 0, 0" "0,0,1" "0,0,1" 0 0))
    ;[1 1 1] If the tear is a piercing tear it doesn't get destroyed after passing through an enemy
    (if (not (Variables|Default|GetPiercing))
      (Actor|DestroyActor))))

(fn ConstructionScript
  (if (not (Variables|Default|GetPiercing))
    (Development|SetHiddeninGame (Variables|Default|GetCone) true false)))